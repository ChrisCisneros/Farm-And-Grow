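; SpawnTrees is a placeable scatter actor that fills a box area with instanced trees from its Construction Script.
; TreeVariation selects one of two meshes for the instanced Tree component, and ScaleContainer sizes the Container box, with a fallback when zero.
; For each of TreeCount attempts, a trace from high above a random box point runs along the actor's down vector against chosen object types.
; Each hit adds an unscaled instance with random yaw.
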(event EventBeginPlay)

(event Collision|EventActorBeginOverlap
  (params (OtherActor :type Actor%20Object%20Reference)))

(event EventTick
  (params (DeltaSeconds :type Float%20%28single-precision%29)))

(fn ConstructionScript
  (bind _container (Variables|Default|GetContainer))
  (bind (_origin _boxextent) (Collision|GetComponentBounds _container))
  (bind _returnvalue (Math|Random|RandomPointinBoundingBox _origin _boxextent))
  (bind (_x _y _z) (Math|Vector|BreakVector _returnvalue))
  (bind _returnvalue_2 (+ _z 1e+05))
  (bind _returnvalue_3 (Math|Vector|MakeVector _x _y _returnvalue_2))
  (Utilities|FlowControl|Sequence
    (:then_0
      (switch int (Variables|Default|GetTree%20Variation)
        (:0
          (Components|StaticMesh|SetStaticMesh (Variables|Default|Gettree) (Variables|Default|GetMesh%20V01)))
        (:1
          (Components|StaticMesh|SetStaticMesh (Variables|Default|Gettree) (Variables|Default|GetMesh%20V02)))))
    (:then_1
      (if (Math|Vector|Equal(Vector) (Variables|Default|GetScaleContainer) "0, 0, 0" 0.0001)
        (Variables|Default|SetScaleContainer "200.000000,200.000000,200.000000"))
      (Components|Box|SetBoxExtent (Variables|Default|GetContainer) (Variables|Default|GetScaleContainer) false)
      (for _index (range 0 (- (Variables|Default|GetTreeCount) 1))
        (bind (_outhit _returnvalue_4) (Collision|LineTraceForObjects _returnvalue_3 (+ _returnvalue_3 (* (* (Transformation|GetActorUpVector) -1) 1.5e+05)) (Variables|Default|GetAttatchToOb) false 0 "None"))
        (if _returnvalue_4
          (Class|InstancedStaticMeshComponent|AddInstanceWorldSpace (Variables|Default|Gettree) (Math|Transform|MakeTransform (.ImpactPoint (Collision|BreakHitResult _outhit)) (Math|Rotator|MakeRotator 0.0 0.0 (Math|Random|RandomFloatinRange 0.0 (Variables|Default|GetMaxRotation))))))))))