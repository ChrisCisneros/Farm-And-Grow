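; Tomato plant Blueprint that advances through visual growth stages from a seed.
; BeginPlay resets the Sections counter, and each Change call increments it up to six.
; The first step toggles visibility on Seed and T1, steps two to five toggle T2 through T5 in turn, and the sixth changes nothing visible.
; A cast of DirtREf to NewBlueprint is left disconnected and never runs.
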(event EventBeginPlay
  (Variables|Default|SetSections 0))

(event Collision|EventActorBeginOverlap
  (params (OtherActor :type Actor%20Object%20Reference)))

(event EventTick
  (params (DeltaSeconds :type Float%20%28single-precision%29)))

(fn ConstructionScript)

(fn Change
  (if (< (Variables|Default|GetSections) 6)
    (Variables|Default|SetSections (+ (Variables|Default|GetSections) 1))
    (if (== 1 (Variables|Default|GetSections))
      (Rendering|ToggleVisibility (Variables|Default|GetSeed) false)
      (Rendering|ToggleVisibility (Variables|Default|GetT1) false)
      (elif (== 2 (Variables|Default|GetSections))
        (Rendering|ToggleVisibility (Variables|Default|GetT2) false)
        (elif (== 3 (Variables|Default|GetSections))
          (Rendering|ToggleVisibility (Variables|Default|GetT3) false)
          (elif (== 4 (Variables|Default|GetSections))
            (Rendering|ToggleVisibility (Variables|Default|GetT4) false)
            (elif (== 5 (Variables|Default|GetSections))
              (Rendering|ToggleVisibility (Variables|Default|GetT5) false))))))))