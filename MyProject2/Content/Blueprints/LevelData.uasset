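; LevelData is an actor that holds the level's clock and money state, setting starting values for both on BeginPlay.
; A looping timer calls Time Advance every ten seconds to add an hour, wrapping to zero after 23 and firing the Change and Dry dispatchers at that rollover.
; Purchase deducts a fixed cost when Money exceeds that amount.
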(event EventBeginPlay
  (Variables|Default|SetHours 9)
  (Variables|Default|SetMoney 15)
  (Utilities|Time|SetTimerbyFunctionName 0 "Time Advance" 1e+01 true))

(event Collision|EventActorBeginOverlap
  (params (OtherActor :type Actor%20Object%20Reference)))

(event EventTick
  (params (DeltaSeconds :type Float%20%28single-precision%29)))

(fn ConstructionScript)

(fn TimeAdvance
  (if (== 23 (Variables|Default|GetHours))
    (Variables|Default|SetHours 0)
    (Default|CallChange)
    (Default|CallDry)
    (else
      (Math|Integer|IncrementInt (Variables|Default|GetHours)))))

(fn Purchase
  (if (> (Variables|Default|GetMoney) 5)
    (Variables|Default|SetMoney (- (Variables|Default|GetMoney) 5))))